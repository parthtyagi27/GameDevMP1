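; ProjectileBP is a player projectile that destroys enemies and awards score.
; Each tick it sweeps along world X faster than the player's ForwardSpeed by a fixed margin, caching the player reference for scoring.
; Sphere hit and overlap events both destroy an EnemyBP and the projectile, but award different points.
; Overlapping any other mesh component destroys only StaticMeshComponent, leaving the projectile actor alive.
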(event OnComponentHit(Sphere)
  (params (HitComponent :type Primitive%20Component%20Object%20Reference) (OtherActor :type Actor%20Object%20Reference) (OtherComp :type Primitive%20Component%20Object%20Reference) (NormalImpulse :type Vector :default "0, 0, 0") (Hit :type Hit%20Result%20Structure%20%28by%20ref%29))
  (bind _playerref (Variables|Default|GetPlayerRef))
  (bind _asenemy_bp (Utilities|Casting|CastToEnemyBP OtherActor))
  (Actor|DestroyActor _asenemy_bp)
  (Variables|/Game/InfiniteMatrix/Blueprints/BP_Player.BP_Player_C|SetScore _playerref (+ (Variables|/Game/InfiniteMatrix/Blueprints/BP_Player.BP_Player_C|GetScore _playerref) 100))
  (Actor|DestroyActor))

(event OnComponentBeginOverlap(Sphere)
  (params (OverlappedComponent :type Primitive%20Component%20Object%20Reference) (OtherActor :type Actor%20Object%20Reference) (OtherComp :type Primitive%20Component%20Object%20Reference) (OtherBodyIndex :type Integer) (bFromSweep :type Boolean) (SweepResult :type Hit%20Result%20Structure%20%28by%20ref%29))
  (bind _playerref (Variables|Default|GetPlayerRef))
  (bind _asenemy_bp (Utilities|Casting|CastToEnemyBP OtherActor)
    (:then
      (Actor|DestroyActor _asenemy_bp)
      (Variables|/Game/InfiniteMatrix/Blueprints/BP_Player.BP_Player_C|SetScore _playerref (+ (Variables|/Game/InfiniteMatrix/Blueprints/BP_Player.BP_Player_C|GetScore _playerref) 3))
      (Actor|DestroyActor))
    (:CastFailed
      (Utilities|Casting|CastToMeshComponent OtherComp)
      (Components|DestroyComponent (Variables|Debug|GetStaticMeshComponent)))))

(event EventBeginPlay)

(event Collision|EventActorBeginOverlap
  (params (OtherActor :type Actor%20Object%20Reference)))

(event EventTick
  (params (DeltaSeconds :type Float%20%28single-precision%29))
  (bind _asbp_player (Utilities|Casting|CastToBP_Player (Game|Player|GetPlayerPawn 0)))
  (Transformation|AddActorWorldOffset (Math|Vector|MakeVector (* DeltaSeconds (+ (Variables|/Game/InfiniteMatrix/Blueprints/BP_Player.BP_Player_C|GetForwardSpeed _asbp_player) 5e+02)) 0.0 0.0) true)
  (Variables|Default|SetPlayerRef _asbp_player))

(fn ConstructionScript)