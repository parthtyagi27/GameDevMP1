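; EnemyBP is an enemy actor that damages the player on contact, with all its logic in the Cone component's hit event.
; Hitting BP_Player lowers Health within clamped bounds, destroys the enemy and deducts Score.
; Zero health calls the player's DisplayRestart, while any other value plays a world camera shake.
; A ProjectileBP hit only prints a debug string and leaves the enemy intact.
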(event OnComponentHit(Cone)
  (params (HitComponent :type Primitive%20Component%20Object%20Reference) (OtherActor :type Actor%20Object%20Reference) (OtherComp :type Primitive%20Component%20Object%20Reference) (NormalImpulse :type Vector :default "0, 0, 0") (Hit :type Hit%20Result%20Structure%20%28by%20ref%29))
  (bind _asbp_player (Utilities|Casting|CastToBP_Player OtherActor)
    (:then
      (bind _output_get (Variables|/Game/InfiniteMatrix/Blueprints/BP_Player.BP_Player_C|SetHealth _asbp_player (Math|Float|Clamp(Float) (- (Variables|/Game/InfiniteMatrix/Blueprints/BP_Player.BP_Player_C|GetHealth _asbp_player) 2e+01) 0.0 1e+02)))
      (Actor|DestroyActor)
      (Variables|/Game/InfiniteMatrix/Blueprints/BP_Player.BP_Player_C|SetScore _asbp_player (- (Variables|/Game/InfiniteMatrix/Blueprints/BP_Player.BP_Player_C|GetScore _asbp_player) 2))
      (if (== _output_get 0.0)
        (Default|DisplayRestart _asbp_player)
        (else
          (Camera|PlayWorldCameraShake "/Script/GameplayCameras.LegacyCameraShake" "0, 0, 0" 0.0 5e+02 1e+02 true)
          (Development|PrintString "shake"))))
    (:CastFailed
      (Utilities|Casting|CastToProjectileBP OtherActor)
      (Development|PrintString "Hello2"))))

(event EventBeginPlay)

(event Collision|EventActorBeginOverlap
  (params (OtherActor :type Actor%20Object%20Reference)))

(event EventTick
  (params (DeltaSeconds :type Float%20%28single-precision%29)))

(fn ConstructionScript)